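; Generated dynamic mesh actor that builds a textured, displaced surface from PCG projection points, bakeable to a static mesh with optional Nanite.
; On rebuild or BeginPlay, each PCG point becomes a rectangle in Geometry Script.
; Optional remeshing solidifies, smooths and unwraps these, clips them to a range sphere, then tessellates and displaces by texture.
; Materials switch between RVT and non-RVT variants, with blend settings driven through a parameter collection.
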(event EventBeginPlay
  (bind _dynamicmeshcomponent (Variables|DynamicMeshActor|GetDynamicMeshComponent))
  (Variables|组件|SetTarget%20Mesh (stale Events|EventOnRebuildGeneratedMesh TargetMesh))
  (Utilities|FlowControl|Sequence
    (:then_0
      (Components|Sphere|SetSphereRadius (Variables|组件|GetSphere) (Variables|BasicSettings|GetRange) true)
      (if (Variables|BasicSettings|GetRefresh)
        _
        (else
          (Variables|BasicSettings|SetRefresh true)))
      (for _array_element (.taggeddata (Class|PCGComponent|GetGeneratedGraphOutput (Variables|组件|GetPCG_MeshProjection)))
        (bind _aspcg点数据 (Utilities|Casting|CastToPCGPointData (.data _array_element)))
        (for _array_element_2 (SpatialData|GetPoints _aspcg点数据)
          (Class|GeometryScriptLibraryMeshPrimitiveFunctions|AppendRoundRectangleXY :TargetMesh (Variables|组件|GetTarget%20Mesh) :Transform (Math|Transform|MakeTransform (- (.location (.transform _array_element_2)) (.location (Transformation|GetActorTransform))) (.rotation (.transform _array_element_2)) "1.000000,1.000000,1.000000") :CornerRadius 0.0 :StepsWidth 5 :StepsHeight 5 :StepsRound 0 :Debug 0))
        (if (Variables|BasicSettings|GetRemesh)
          (bind _returnvalue (Class|GeometryScriptLibraryMeshVoxelFunctions|ApplyMeshSolidify (Variables|组件|GetTarget%20Mesh) (Utilities|Struct|MakeGeometryScriptSolidifyOptions (Utilities|Struct|MakeGeometryScript3DGridParameters "GridResolution" 0.0 32) 0.0 false 4.0 2 false 0.0) 0))
          (bind _returnvalue_2 (Class|GeometryScriptLibraryMeshDeformFunctions|ApplyIterativeSmoothingtoMesh :TargetMesh _returnvalue :Options (Utilities|Struct|MakeGeometryScriptIterativeMeshSmoothingOptions (Variables|BasicSettings|GetSmooth) 0.2 "FullMeshSelection") :Debug 0))
          (bind _returnvalue_3 (Class|GeometryScriptLibraryMeshUVFunctions|AutoGenerateXAtlasMeshUVs _returnvalue_2 0 (Utilities|Struct|MakeGeometryScriptXAtlasOptions 1) 0))
          (bind _returnvalue_4 (Class|GeometryScriptLibraryMeshDeformFunctions|ApplyDisplacefromTextureMap :TargetMesh _returnvalue_3 :Texture (.As纹理2D (Utilities|Casting|CastToTexture2D (Variables|组件|GetSphere_Mask))) :Options (Utilities|Struct|MakeGeometryScriptDisplaceFromTextureOptions (* (Variables|BasicSettings|GetEdge_Z_Offset) -1.0) "(X=1.000000,Y=-1.000000)" "(X=0.000000,Y=0.000000)" 0.5 0 "FullMeshSelection") :Debug 0))
          (bind _returnvalue_5 (Class|GeometryScriptLibraryMeshNormalsFunctions|ComputeTangents :TargetMesh _returnvalue_4 :Debug 0))
          (bind _returnvalue_6 (DynamicMeshActor|AllocateComputeMesh))
          (bind _returnvalue_7 (Class|GeometryScriptLibraryMeshPrimitiveFunctions|AppendSphereBox :TargetMesh _returnvalue_6 :Radius (Variables|BasicSettings|GetRange) :StepsX 15 :StepsY 15 :StepsZ 15 :Debug 0))
          (bind _returnvalue_8 (GeometryScript|Booleans|ApplyMeshBoolean :TargetMesh _returnvalue_5 :ToolMesh _returnvalue_7 :Operation "Intersection" :Options (Utilities|Struct|MakeGeometryScriptMeshBooleanOptions false true 0.01 true) :Debug 0))
          (bind _returnvalue_9 (GeometryScript|UVs|ScaleMeshUVs :TargetMesh _returnvalue_8 :Scale (Variables|MeshMaterial|GetScale_UV) :ScaleOrigin "(X=0.000000,Y=0.000000)" :Debug 0))
          (bind _returnvalue_10 (Class|GeometryScriptLibraryMeshUVFunctions|RotateMeshUVs :TargetMesh _returnvalue_9 :RotationAngle (Variables|MeshMaterial|GetRotation_UV) :Debug 0))
          (bind _returnvalue_11 (Class|GeometryScriptLibraryMeshNormalsFunctions|ComputeSplitNormals :TargetMesh _returnvalue_10 :SplitOptions (Utilities|Struct|MakeGeometryScriptSplitNormalsOptions true 9e+01 false "(bDefaultLayer=True,ExtendedLayerIndex=0)") :Debug 0))
          (Class|GeometryScriptLibraryMeshSubdivideFunctions|ApplyUniformTessellation _returnvalue_11 (Variables|MeshMaterial|GetDisplace_Steps) 0)
          (Class|GeometryScriptLibraryMeshDeformFunctions|ApplyDisplacefromTextureMap :TargetMesh (Variables|组件|GetTarget%20Mesh) :Texture (.As纹理2D (Utilities|Casting|CastToTexture2D (Variables|MeshMaterial|GetDisplace_Texture))) :Options (Utilities|Struct|MakeGeometryScriptDisplaceFromTextureOptions (Variables|MeshMaterial|GetDisplace_Intensity) "(X=1.000000,Y=1.000000)" "(X=0.000000,Y=0.000000)" 0.0 (.Value (Utilities|Map|Find (Variables|组件|GetTexture_Channel) (Variables|MeshMaterial|GetDisplace_Channel))) "FullMeshSelection") :Debug 0))))
    (:then_1
      (if (Variables|MeshMaterial|GetUse_RVT?)
        (Rendering|Material|SetScalarParameterValue "/Game/Natural_PCGTools/PCG/Other/MPC_MeshProjection.MPC_MeshProjection" "DetermineRVT" 1.0 :!class /Script/Engine.KismetMaterialLibrary)
        (Rendering|Material|SetMaterial (Variables|DynamicMeshActor|GetDynamicMeshComponent) 0 (Variables|MeshMaterial|GetMesh_Material_RVT))
        (Class|MaterialEditingLibrary|SetMaterialInstanceRuntimeVirtualTextureParameterValue (Variables|OtherSettings|GetBake_Material) "RVT_BaseColor" (Variables|MeshMaterial|GetRVT_BaseColor) "GlobalParameter")
        (if (not (Variables|OtherSettings|GetCustom_Materials))
          (Variables|OtherSettings|SetBake_Material (Variables|MeshMaterial|GetMesh_Material_RVT)))
        (else
          (Rendering|Material|SetScalarParameterValue "/Game/Natural_PCGTools/PCG/Other/MPC_MeshProjection.MPC_MeshProjection" "DetermineRVT" 0.0 :!class /Script/Engine.KismetMaterialLibrary)
          (Rendering|Material|SetMaterial (Variables|DynamicMeshActor|GetDynamicMeshComponent) 0 (Variables|MeshMaterial|GetMesh_Material_NoRVT))
          (if (not (Variables|OtherSettings|GetCustom_Materials))
            (Variables|OtherSettings|SetBake_Material (Variables|MeshMaterial|GetMesh_Material_NoRVT))))))
    (:then_2
      (GeometryScript|Transforms|TransformMesh (Variables|组件|GetTarget%20Mesh) (Math|Transform|MakeTransform (Math|Vector|MakeVector 0.0 0.0 (Variables|BasicSettings|GetGlobal_Z_Offset)) "0, 0, 0" "1.000000,1.000000,1.000000") true 0)
      (bind _returnvalue_12 (Rendering|Material|CreateDynamicMaterialInstance _dynamicmeshcomponent 0 (Rendering|Material|GetMaterial _dynamicmeshcomponent 0) "None" :!class /Script/Engine.PrimitiveComponent))
      (Rendering|Material|SetTextureParameterValue _returnvalue_12 "BaseColor_Texture" (Variables|MeshMaterial|GetBaseColor_Texture))
      (Rendering|Material|SetTextureParameterValue _returnvalue_12 "Normal_Texture" (Variables|MeshMaterial|GetNormal_Texture))
      (Rendering|Material|SetTextureParameterValue _returnvalue_12 "Displace_Texture" (Variables|MeshMaterial|GetDisplace_Texture))
      (Rendering|Material|SetScalarParameterValue "/Game/Natural_PCGTools/PCG/Other/MPC_MeshProjection.MPC_MeshProjection" "RVT_Range" (Variables|MeshMaterial|GetRVT_Range) :!class /Script/Engine.KismetMaterialLibrary)
      (Rendering|Material|SetScalarParameterValue "/Game/Natural_PCGTools/PCG/Other/MPC_MeshProjection.MPC_MeshProjection" "RVT_Contrast" (Variables|MeshMaterial|GetRVT_Contrast) :!class /Script/Engine.KismetMaterialLibrary))))

(event Collision|EventActorBeginOverlap
  (params (OtherActor :type Actor%20Object%20Reference)))

(event EventTick
  (params (DeltaSeconds :type Float%20%28single-precision%29)))

(event Events|EventOnRebuildGeneratedMesh
  (params (TargetMesh :type Dynamic%20Mesh%20Object%20Reference))
  (bind _dynamicmeshcomponent (Variables|DynamicMeshActor|GetDynamicMeshComponent))
  (Variables|组件|SetTarget%20Mesh TargetMesh)
  (Utilities|FlowControl|Sequence
    (:then_0
      (Components|Sphere|SetSphereRadius (Variables|组件|GetSphere) (Variables|BasicSettings|GetRange) true)
      (if (Variables|BasicSettings|GetRefresh)
        _
        (else
          (Variables|BasicSettings|SetRefresh true)))
      (for _array_element (.taggeddata (Class|PCGComponent|GetGeneratedGraphOutput (Variables|组件|GetPCG_MeshProjection)))
        (bind _aspcg点数据 (Utilities|Casting|CastToPCGPointData (.data _array_element)))
        (for _array_element_2 (SpatialData|GetPoints _aspcg点数据)
          (Class|GeometryScriptLibraryMeshPrimitiveFunctions|AppendRoundRectangleXY :TargetMesh (Variables|组件|GetTarget%20Mesh) :Transform (Math|Transform|MakeTransform (- (.location (.transform _array_element_2)) (.location (Transformation|GetActorTransform))) (.rotation (.transform _array_element_2)) "1.000000,1.000000,1.000000") :CornerRadius 0.0 :StepsWidth 5 :StepsHeight 5 :StepsRound 0 :Debug 0))
        (if (Variables|BasicSettings|GetRemesh)
          (bind _returnvalue (Class|GeometryScriptLibraryMeshVoxelFunctions|ApplyMeshSolidify (Variables|组件|GetTarget%20Mesh) (Utilities|Struct|MakeGeometryScriptSolidifyOptions (Utilities|Struct|MakeGeometryScript3DGridParameters "GridResolution" 0.0 32) 0.0 false 4.0 2 false 0.0) 0))
          (bind _returnvalue_2 (Class|GeometryScriptLibraryMeshDeformFunctions|ApplyIterativeSmoothingtoMesh :TargetMesh _returnvalue :Options (Utilities|Struct|MakeGeometryScriptIterativeMeshSmoothingOptions (Variables|BasicSettings|GetSmooth) 0.2 "FullMeshSelection") :Debug 0))
          (bind _returnvalue_3 (Class|GeometryScriptLibraryMeshUVFunctions|AutoGenerateXAtlasMeshUVs _returnvalue_2 0 (Utilities|Struct|MakeGeometryScriptXAtlasOptions 1) 0))
          (bind _returnvalue_4 (Class|GeometryScriptLibraryMeshDeformFunctions|ApplyDisplacefromTextureMap :TargetMesh _returnvalue_3 :Texture (.As纹理2D (Utilities|Casting|CastToTexture2D (Variables|组件|GetSphere_Mask))) :Options (Utilities|Struct|MakeGeometryScriptDisplaceFromTextureOptions (* (Variables|BasicSettings|GetEdge_Z_Offset) -1.0) "(X=1.000000,Y=-1.000000)" "(X=0.000000,Y=0.000000)" 0.5 0 "FullMeshSelection") :Debug 0))
          (bind _returnvalue_5 (Class|GeometryScriptLibraryMeshNormalsFunctions|ComputeTangents :TargetMesh _returnvalue_4 :Debug 0))
          (bind _returnvalue_6 (DynamicMeshActor|AllocateComputeMesh))
          (bind _returnvalue_7 (Class|GeometryScriptLibraryMeshPrimitiveFunctions|AppendSphereBox :TargetMesh _returnvalue_6 :Radius (Variables|BasicSettings|GetRange) :StepsX 15 :StepsY 15 :StepsZ 15 :Debug 0))
          (bind _returnvalue_8 (GeometryScript|Booleans|ApplyMeshBoolean :TargetMesh _returnvalue_5 :ToolMesh _returnvalue_7 :Operation "Intersection" :Options (Utilities|Struct|MakeGeometryScriptMeshBooleanOptions false true 0.01 true) :Debug 0))
          (bind _returnvalue_9 (GeometryScript|UVs|ScaleMeshUVs :TargetMesh _returnvalue_8 :Scale (Variables|MeshMaterial|GetScale_UV) :ScaleOrigin "(X=0.000000,Y=0.000000)" :Debug 0))
          (bind _returnvalue_10 (Class|GeometryScriptLibraryMeshUVFunctions|RotateMeshUVs :TargetMesh _returnvalue_9 :RotationAngle (Variables|MeshMaterial|GetRotation_UV) :Debug 0))
          (bind _returnvalue_11 (Class|GeometryScriptLibraryMeshNormalsFunctions|ComputeSplitNormals :TargetMesh _returnvalue_10 :SplitOptions (Utilities|Struct|MakeGeometryScriptSplitNormalsOptions true 9e+01 false "(bDefaultLayer=True,ExtendedLayerIndex=0)") :Debug 0))
          (Class|GeometryScriptLibraryMeshSubdivideFunctions|ApplyUniformTessellation _returnvalue_11 (Variables|MeshMaterial|GetDisplace_Steps) 0)
          (Class|GeometryScriptLibraryMeshDeformFunctions|ApplyDisplacefromTextureMap :TargetMesh (Variables|组件|GetTarget%20Mesh) :Texture (.As纹理2D (Utilities|Casting|CastToTexture2D (Variables|MeshMaterial|GetDisplace_Texture))) :Options (Utilities|Struct|MakeGeometryScriptDisplaceFromTextureOptions (Variables|MeshMaterial|GetDisplace_Intensity) "(X=1.000000,Y=1.000000)" "(X=0.000000,Y=0.000000)" 0.0 (.Value (Utilities|Map|Find (Variables|组件|GetTexture_Channel) (Variables|MeshMaterial|GetDisplace_Channel))) "FullMeshSelection") :Debug 0))))
    (:then_1
      (if (Variables|MeshMaterial|GetUse_RVT?)
        (Rendering|Material|SetScalarParameterValue "/Game/Natural_PCGTools/PCG/Other/MPC_MeshProjection.MPC_MeshProjection" "DetermineRVT" 1.0 :!class /Script/Engine.KismetMaterialLibrary)
        (Rendering|Material|SetMaterial (Variables|DynamicMeshActor|GetDynamicMeshComponent) 0 (Variables|MeshMaterial|GetMesh_Material_RVT))
        (Class|MaterialEditingLibrary|SetMaterialInstanceRuntimeVirtualTextureParameterValue (Variables|OtherSettings|GetBake_Material) "RVT_BaseColor" (Variables|MeshMaterial|GetRVT_BaseColor) "GlobalParameter")
        (if (not (Variables|OtherSettings|GetCustom_Materials))
          (Variables|OtherSettings|SetBake_Material (Variables|MeshMaterial|GetMesh_Material_RVT)))
        (else
          (Rendering|Material|SetScalarParameterValue "/Game/Natural_PCGTools/PCG/Other/MPC_MeshProjection.MPC_MeshProjection" "DetermineRVT" 0.0 :!class /Script/Engine.KismetMaterialLibrary)
          (Rendering|Material|SetMaterial (Variables|DynamicMeshActor|GetDynamicMeshComponent) 0 (Variables|MeshMaterial|GetMesh_Material_NoRVT))
          (if (not (Variables|OtherSettings|GetCustom_Materials))
            (Variables|OtherSettings|SetBake_Material (Variables|MeshMaterial|GetMesh_Material_NoRVT))))))
    (:then_2
      (GeometryScript|Transforms|TransformMesh (Variables|组件|GetTarget%20Mesh) (Math|Transform|MakeTransform (Math|Vector|MakeVector 0.0 0.0 (Variables|BasicSettings|GetGlobal_Z_Offset)) "0, 0, 0" "1.000000,1.000000,1.000000") true 0)
      (bind _returnvalue_12 (Rendering|Material|CreateDynamicMaterialInstance _dynamicmeshcomponent 0 (Rendering|Material|GetMaterial _dynamicmeshcomponent 0) "None" :!class /Script/Engine.PrimitiveComponent))
      (Rendering|Material|SetTextureParameterValue _returnvalue_12 "BaseColor_Texture" (Variables|MeshMaterial|GetBaseColor_Texture))
      (Rendering|Material|SetTextureParameterValue _returnvalue_12 "Normal_Texture" (Variables|MeshMaterial|GetNormal_Texture))
      (Rendering|Material|SetTextureParameterValue _returnvalue_12 "Displace_Texture" (Variables|MeshMaterial|GetDisplace_Texture))
      (Rendering|Material|SetScalarParameterValue "/Game/Natural_PCGTools/PCG/Other/MPC_MeshProjection.MPC_MeshProjection" "RVT_Range" (Variables|MeshMaterial|GetRVT_Range) :!class /Script/Engine.KismetMaterialLibrary)
      (Rendering|Material|SetScalarParameterValue "/Game/Natural_PCGTools/PCG/Other/MPC_MeshProjection.MPC_MeshProjection" "RVT_Contrast" (Variables|MeshMaterial|GetRVT_Contrast) :!class /Script/Engine.KismetMaterialLibrary))))

(fn ConstructionScript)

(fn BaketoMesh
  (bind _bake_material (Variables|OtherSettings|GetBake_Material))
  (bind _returnvalue (DynamicMeshComponent|GetDynamicMesh (Variables|DynamicMeshActor|GetDynamicMeshComponent)))
  (GeometryScript|StaticMesh|CopyMeshtoStaticMesh :FromDynamicMesh _returnvalue :ToStaticMeshAsset (Variables|OtherSettings|GetStatic_Mesh_Asset) :Options (Utilities|Struct|MakeGeometryScriptCopyMeshtoAssetOptions true true true false true true (Utilities|IsValid _bake_material) (Utilities|Array|MakeArray _bake_material) (Utilities|Array|MakeArray "MeshProjection") true "(bEnabled=True,FallbackPercentTriangles=100.000000,FallbackRelativeError=0.000000)" (Utilities|Struct|MakeMeshNaniteSettings (Variables|OtherSettings|GetNanite) false false true -2147483648 -1 -1 1.0 0.0 "Auto" 1.0 1.0 0.0 0) true false) :Debug 0))