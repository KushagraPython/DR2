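; Generated dynamic mesh actor that builds a snow layer from PCG points and can bake it to a static mesh, optionally Nanite.
; On mesh rebuild or BeginPlay, it appends thickness-scaled sphere boxes at each PCGSnowProjection point.
; Optional remeshing merges them through morphology, box-projected UVs, Perlin noise and smoothing, with optional tessellated texture displacement afterwards.
; An RVT switch selects the material and drives the MPC_Mesh_Snow parameter collection.
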(event EventBeginPlay
  (bind _dynamicmeshcomponent (Variables|DynamicMeshActor|GetDynamicMeshComponent))
  (bind _pcg_range (Variables|组件|GetPCG_Range))
  (bind _scale_uv (Variables|MeshMaterial|GetScale_UV))
  (bind _displace_uvscale (Variables|MeshMaterial|GetDisplace_UVScale))
  (bind _returnvalue (* _scale_uv 1e+01))
  (bind _returnvalue_2 (/ _displace_uvscale 1e+01))
  (Variables|组件|SetTarget%20Mesh (stale Events|EventOnRebuildGeneratedMesh TargetMesh))
  (Utilities|FlowControl|Sequence
    (:then_0
      (Components|Box|SetBoxExtent (Variables|Default|GetBox) (Math|Vector|MakeVector _pcg_range _pcg_range _pcg_range) true)
      (if (Variables|BasicSettings|GetRefresh)
        _
        (else
          (Variables|BasicSettings|SetRefresh true)))
      (for _array_element (.taggeddata (Class|PCGComponent|GetGeneratedGraphOutput (Variables|组件|GetPCG_SnowProjection)))
        (bind _aspcgpoint_data (Utilities|Casting|CastToPCGPointData (.data _array_element)))
        (for _array_element_2 (SpatialData|GetPoints _aspcgpoint_data)
          (Class|GeometryScriptLibraryMeshPrimitiveFunctions|AppendSphereBox :TargetMesh (Variables|组件|GetTarget%20Mesh) :Transform (Math|Transform|MakeTransform (- (.location (.transform _array_element_2)) (.location (Transformation|GetActorTransform))) (.rotation (.transform _array_element_2)) (Math|Vector|MakeVector 1.0 1.0 (Variables|BasicSettings|GetSnow_Thickness))) :Radius (Variables|BasicSettings|GetRadius) :StepsX 4 :StepsY 4 :StepsZ 4 :Debug 0))
        (if (Variables|BasicSettings|GetRemesh)
          (bind _returnvalue_3 (Class|GeometryScriptLibraryMeshVoxelFunctions|ApplyMeshMorphology (Variables|组件|GetTarget%20Mesh) (Utilities|Struct|MakeGeometryScriptMorphologyOptions (Utilities|Struct|MakeGeometryScript3DGridParameters "GridResolution" 0.5 150) false (Utilities|Struct|MakeGeometryScript3DGridParameters "GridResolution" 0.5 32) "Dilate" (* (Variables|BasicSettings|GetSnow_Thickness) 1e+01)) 0))
          (bind _returnvalue_4 (Class|GeometryScriptLibraryMeshUVFunctions|SetMeshUVsfromBoxProjection :TargetMesh _returnvalue_3 :BoxTransform (Math|Transform|MakeTransform "0, 0, 0" "0, 0, 0" (Math|Vector|MakeVector _returnvalue _returnvalue _returnvalue)) :Debug 0))
          (bind _returnvalue_5 (Class|GeometryScriptLibraryMeshUVFunctions|RotateMeshUVs :TargetMesh _returnvalue_4 :RotationAngle (Variables|MeshMaterial|GetRotation_UV) :Debug 0))
          (bind _returnvalue_6 (Class|GeometryScriptLibraryMeshDeformFunctions|ApplyPerlinNoisetoMesh :TargetMesh _returnvalue_5 :Options (Utilities|Struct|MakeGeometryScriptPerlinNoiseOptions (Utilities|Struct|MakeGeometryScriptPerlinNoiseLayerOptions (Variables|BasicSettings|GetNoise_Intensity) (/ 1.0 (Variables|BasicSettings|GetNoise_UV)) "0.000000,0.000000,0.000000" (Variables|BasicSettings|GetRandom_Seed)) true "FullMeshSelection") :Debug 0))
          (bind _returnvalue_7 (Class|GeometryScriptLibraryMeshDeformFunctions|ApplyIterativeSmoothingtoMesh :TargetMesh _returnvalue_6 :Options (Utilities|Struct|MakeGeometryScriptIterativeMeshSmoothingOptions (Variables|BasicSettings|GetSmooth) 0.4 "FullMeshSelection") :Debug 0))
          (bind _returnvalue_8 (Class|GeometryScriptLibraryMeshNormalsFunctions|ComputeTangents :TargetMesh _returnvalue_7 :Debug 0))
          (Class|GeometryScriptLibraryMeshNormalsFunctions|ComputeSplitNormals _returnvalue_8 (Utilities|Struct|MakeGeometryScriptSplitNormalsOptions true 9e+01 false "(bDefaultLayer=True,ExtendedLayerIndex=0)") (Utilities|Struct|MakeGeometryScriptCalculateNormalsOptions true true) 0))))
    (:then_1
      (if (Variables|MeshMaterial|GetUse_RVT?)
        (Rendering|Material|SetScalarParameterValue "/Game/Natural_PCGTools/PCG/Other/MPC_Mesh_Snow.MPC_Mesh_Snow" "DetermineRVT" 1.0 :!class /Script/Engine.KismetMaterialLibrary)
        (Rendering|Material|SetMaterial (Variables|DynamicMeshActor|GetDynamicMeshComponent) 0 (Variables|MeshMaterial|GetMesh_Material_RVT))
        (Class|MaterialEditingLibrary|SetMaterialInstanceRuntimeVirtualTextureParameterValue (Variables|OtherSettings|GetBake_Material) "RVT_BaseColor" (Variables|MeshMaterial|GetRVT_BaseColor) "GlobalParameter")
        (if (not (Variables|OtherSettings|GetCustom_Materials))
          (Variables|OtherSettings|SetBake_Material (Variables|MeshMaterial|GetMesh_Material_RVT)))
        (else
          (Rendering|Material|SetScalarParameterValue "/Game/Natural_PCGTools/PCG/Other/MPC_Mesh_Snow.MPC_Mesh_Snow" "DetermineRVT" 0.0 :!class /Script/Engine.KismetMaterialLibrary)
          (Rendering|Material|SetMaterial (Variables|DynamicMeshActor|GetDynamicMeshComponent) 0 (Variables|MeshMaterial|GetMesh_Material_NoRVT))
          (if (not (Variables|OtherSettings|GetCustom_Materials))
            (Variables|OtherSettings|SetBake_Material (Variables|MeshMaterial|GetMesh_Material_NoRVT))))))
    (:then_2
      (GeometryScript|Transforms|TransformMesh (Variables|组件|GetTarget%20Mesh) (Math|Transform|MakeTransform (Math|Vector|MakeVector 0.0 0.0 (Variables|BasicSettings|GetGlobal_Z_Offset)) "0, 0, 0" "1.000000,1.000000,1.000000") true 0)
      (if (Variables|MeshMaterial|GetUse_Displace_Texture)
        (bind _returnvalue_9 (Class|GeometryScriptLibraryMeshSubdivideFunctions|ApplyPNTessellation (Variables|组件|GetTarget%20Mesh) (Utilities|Struct|MakeGeometryScriptPNTessellateOptions true) (Variables|MeshMaterial|GetDisplace_Steps) 0))
        (Class|GeometryScriptLibraryMeshDeformFunctions|ApplyDisplacefromTextureMap :TargetMesh _returnvalue_9 :Texture (.AsTexture%202D (Utilities|Casting|CastToTexture2D (Variables|MeshMaterial|GetDisplace_Texture))) :Options (Utilities|Struct|MakeGeometryScriptDisplaceFromTextureOptions (Variables|MeshMaterial|GetDisplace_Intensity) (Math|Vector2D|MakeVector2D _returnvalue_2 _returnvalue_2) "(X=0.000000,Y=0.000000)" 0.0 (.Value (Utilities|Map|Find (Variables|组件|GetTexture_Channel) (Variables|MeshMaterial|GetDisplace_Channel))) "FullMeshSelection") :Debug 0))
      (bind _returnvalue_10 (Rendering|Material|CreateDynamicMaterialInstance _dynamicmeshcomponent 0 (Rendering|Material|GetMaterial _dynamicmeshcomponent 0) "None" :!class /Script/Engine.PrimitiveComponent))
      (Rendering|Material|SetTextureParameterValue _returnvalue_10 "BaseColor_Texture" (Variables|MeshMaterial|GetBaseColor_Texture))
      (Rendering|Material|SetTextureParameterValue _returnvalue_10 "Normal_Texture" (Variables|MeshMaterial|GetNormal_Texture))
      (Rendering|Material|SetTextureParameterValue _returnvalue_10 "Displace_Texture" (Variables|MeshMaterial|GetDisplace_Texture))
      (Rendering|Material|SetScalarParameterValue "/Game/Natural_PCGTools/PCG/Other/MPC_Mesh_Snow.MPC_Mesh_Snow" "RVT_Range" (Variables|MeshMaterial|GetRVT_Range) :!class /Script/Engine.KismetMaterialLibrary)
      (Rendering|Material|SetScalarParameterValue "/Game/Natural_PCGTools/PCG/Other/MPC_Mesh_Snow.MPC_Mesh_Snow" "RVT_Contrast" (Variables|MeshMaterial|GetRVT_Contrast) :!class /Script/Engine.KismetMaterialLibrary))))

(event Collision|EventActorBeginOverlap
  (params (OtherActor :type Actor%20Object%20Reference)))

(event EventTick
  (params (DeltaSeconds :type Float%20%28single-precision%29)))

(event Events|EventOnRebuildGeneratedMesh
  (params (TargetMesh :type Dynamic%20Mesh%20Object%20Reference))
  (bind _dynamicmeshcomponent (Variables|DynamicMeshActor|GetDynamicMeshComponent))
  (bind _pcg_range (Variables|组件|GetPCG_Range))
  (bind _scale_uv (Variables|MeshMaterial|GetScale_UV))
  (bind _displace_uvscale (Variables|MeshMaterial|GetDisplace_UVScale))
  (bind _returnvalue (* _scale_uv 1e+01))
  (bind _returnvalue_2 (/ _displace_uvscale 1e+01))
  (Variables|组件|SetTarget%20Mesh TargetMesh)
  (Utilities|FlowControl|Sequence
    (:then_0
      (Components|Box|SetBoxExtent (Variables|Default|GetBox) (Math|Vector|MakeVector _pcg_range _pcg_range _pcg_range) true)
      (if (Variables|BasicSettings|GetRefresh)
        _
        (else
          (Variables|BasicSettings|SetRefresh true)))
      (for _array_element (.taggeddata (Class|PCGComponent|GetGeneratedGraphOutput (Variables|组件|GetPCG_SnowProjection)))
        (bind _aspcgpoint_data (Utilities|Casting|CastToPCGPointData (.data _array_element)))
        (for _array_element_2 (SpatialData|GetPoints _aspcgpoint_data)
          (Class|GeometryScriptLibraryMeshPrimitiveFunctions|AppendSphereBox :TargetMesh (Variables|组件|GetTarget%20Mesh) :Transform (Math|Transform|MakeTransform (- (.location (.transform _array_element_2)) (.location (Transformation|GetActorTransform))) (.rotation (.transform _array_element_2)) (Math|Vector|MakeVector 1.0 1.0 (Variables|BasicSettings|GetSnow_Thickness))) :Radius (Variables|BasicSettings|GetRadius) :StepsX 4 :StepsY 4 :StepsZ 4 :Debug 0))
        (if (Variables|BasicSettings|GetRemesh)
          (bind _returnvalue_3 (Class|GeometryScriptLibraryMeshVoxelFunctions|ApplyMeshMorphology (Variables|组件|GetTarget%20Mesh) (Utilities|Struct|MakeGeometryScriptMorphologyOptions (Utilities|Struct|MakeGeometryScript3DGridParameters "GridResolution" 0.5 150) false (Utilities|Struct|MakeGeometryScript3DGridParameters "GridResolution" 0.5 32) "Dilate" (* (Variables|BasicSettings|GetSnow_Thickness) 1e+01)) 0))
          (bind _returnvalue_4 (Class|GeometryScriptLibraryMeshUVFunctions|SetMeshUVsfromBoxProjection :TargetMesh _returnvalue_3 :BoxTransform (Math|Transform|MakeTransform "0, 0, 0" "0, 0, 0" (Math|Vector|MakeVector _returnvalue _returnvalue _returnvalue)) :Debug 0))
          (bind _returnvalue_5 (Class|GeometryScriptLibraryMeshUVFunctions|RotateMeshUVs :TargetMesh _returnvalue_4 :RotationAngle (Variables|MeshMaterial|GetRotation_UV) :Debug 0))
          (bind _returnvalue_6 (Class|GeometryScriptLibraryMeshDeformFunctions|ApplyPerlinNoisetoMesh :TargetMesh _returnvalue_5 :Options (Utilities|Struct|MakeGeometryScriptPerlinNoiseOptions (Utilities|Struct|MakeGeometryScriptPerlinNoiseLayerOptions (Variables|BasicSettings|GetNoise_Intensity) (/ 1.0 (Variables|BasicSettings|GetNoise_UV)) "0.000000,0.000000,0.000000" (Variables|BasicSettings|GetRandom_Seed)) true "FullMeshSelection") :Debug 0))
          (bind _returnvalue_7 (Class|GeometryScriptLibraryMeshDeformFunctions|ApplyIterativeSmoothingtoMesh :TargetMesh _returnvalue_6 :Options (Utilities|Struct|MakeGeometryScriptIterativeMeshSmoothingOptions (Variables|BasicSettings|GetSmooth) 0.4 "FullMeshSelection") :Debug 0))
          (bind _returnvalue_8 (Class|GeometryScriptLibraryMeshNormalsFunctions|ComputeTangents :TargetMesh _returnvalue_7 :Debug 0))
          (Class|GeometryScriptLibraryMeshNormalsFunctions|ComputeSplitNormals _returnvalue_8 (Utilities|Struct|MakeGeometryScriptSplitNormalsOptions true 9e+01 false "(bDefaultLayer=True,ExtendedLayerIndex=0)") (Utilities|Struct|MakeGeometryScriptCalculateNormalsOptions true true) 0))))
    (:then_1
      (if (Variables|MeshMaterial|GetUse_RVT?)
        (Rendering|Material|SetScalarParameterValue "/Game/Natural_PCGTools/PCG/Other/MPC_Mesh_Snow.MPC_Mesh_Snow" "DetermineRVT" 1.0 :!class /Script/Engine.KismetMaterialLibrary)
        (Rendering|Material|SetMaterial (Variables|DynamicMeshActor|GetDynamicMeshComponent) 0 (Variables|MeshMaterial|GetMesh_Material_RVT))
        (Class|MaterialEditingLibrary|SetMaterialInstanceRuntimeVirtualTextureParameterValue (Variables|OtherSettings|GetBake_Material) "RVT_BaseColor" (Variables|MeshMaterial|GetRVT_BaseColor) "GlobalParameter")
        (if (not (Variables|OtherSettings|GetCustom_Materials))
          (Variables|OtherSettings|SetBake_Material (Variables|MeshMaterial|GetMesh_Material_RVT)))
        (else
          (Rendering|Material|SetScalarParameterValue "/Game/Natural_PCGTools/PCG/Other/MPC_Mesh_Snow.MPC_Mesh_Snow" "DetermineRVT" 0.0 :!class /Script/Engine.KismetMaterialLibrary)
          (Rendering|Material|SetMaterial (Variables|DynamicMeshActor|GetDynamicMeshComponent) 0 (Variables|MeshMaterial|GetMesh_Material_NoRVT))
          (if (not (Variables|OtherSettings|GetCustom_Materials))
            (Variables|OtherSettings|SetBake_Material (Variables|MeshMaterial|GetMesh_Material_NoRVT))))))
    (:then_2
      (GeometryScript|Transforms|TransformMesh (Variables|组件|GetTarget%20Mesh) (Math|Transform|MakeTransform (Math|Vector|MakeVector 0.0 0.0 (Variables|BasicSettings|GetGlobal_Z_Offset)) "0, 0, 0" "1.000000,1.000000,1.000000") true 0)
      (if (Variables|MeshMaterial|GetUse_Displace_Texture)
        (bind _returnvalue_9 (Class|GeometryScriptLibraryMeshSubdivideFunctions|ApplyPNTessellation (Variables|组件|GetTarget%20Mesh) (Utilities|Struct|MakeGeometryScriptPNTessellateOptions true) (Variables|MeshMaterial|GetDisplace_Steps) 0))
        (Class|GeometryScriptLibraryMeshDeformFunctions|ApplyDisplacefromTextureMap :TargetMesh _returnvalue_9 :Texture (.AsTexture%202D (Utilities|Casting|CastToTexture2D (Variables|MeshMaterial|GetDisplace_Texture))) :Options (Utilities|Struct|MakeGeometryScriptDisplaceFromTextureOptions (Variables|MeshMaterial|GetDisplace_Intensity) (Math|Vector2D|MakeVector2D _returnvalue_2 _returnvalue_2) "(X=0.000000,Y=0.000000)" 0.0 (.Value (Utilities|Map|Find (Variables|组件|GetTexture_Channel) (Variables|MeshMaterial|GetDisplace_Channel))) "FullMeshSelection") :Debug 0))
      (bind _returnvalue_10 (Rendering|Material|CreateDynamicMaterialInstance _dynamicmeshcomponent 0 (Rendering|Material|GetMaterial _dynamicmeshcomponent 0) "None" :!class /Script/Engine.PrimitiveComponent))
      (Rendering|Material|SetTextureParameterValue _returnvalue_10 "BaseColor_Texture" (Variables|MeshMaterial|GetBaseColor_Texture))
      (Rendering|Material|SetTextureParameterValue _returnvalue_10 "Normal_Texture" (Variables|MeshMaterial|GetNormal_Texture))
      (Rendering|Material|SetTextureParameterValue _returnvalue_10 "Displace_Texture" (Variables|MeshMaterial|GetDisplace_Texture))
      (Rendering|Material|SetScalarParameterValue "/Game/Natural_PCGTools/PCG/Other/MPC_Mesh_Snow.MPC_Mesh_Snow" "RVT_Range" (Variables|MeshMaterial|GetRVT_Range) :!class /Script/Engine.KismetMaterialLibrary)
      (Rendering|Material|SetScalarParameterValue "/Game/Natural_PCGTools/PCG/Other/MPC_Mesh_Snow.MPC_Mesh_Snow" "RVT_Contrast" (Variables|MeshMaterial|GetRVT_Contrast) :!class /Script/Engine.KismetMaterialLibrary))))

(fn ConstructionScript)

(fn BaketoMesh
  (bind _bake_material (Variables|OtherSettings|GetBake_Material))
  (bind _returnvalue (DynamicMeshComponent|GetDynamicMesh (Variables|DynamicMeshActor|GetDynamicMeshComponent)))
  (GeometryScript|StaticMesh|CopyMeshtoStaticMesh :FromDynamicMesh _returnvalue :ToStaticMeshAsset (Variables|OtherSettings|GetStatic_Mesh_Asset) :Options (Utilities|Struct|MakeGeometryScriptCopyMeshtoAssetOptions true true true false true true (Utilities|IsValid _bake_material) (Utilities|Array|MakeArray _bake_material) (Utilities|Array|MakeArray "Snow") true "(bEnabled=True,FallbackPercentTriangles=100.000000,FallbackRelativeError=0.000000)" (Utilities|Struct|MakeMeshNaniteSettings (Variables|OtherSettings|GetNanite) false false true -2147483648 -1 -1 1.0 0.0 "Auto" 1.0 1.0 0.0 0) true false) :Debug 0))