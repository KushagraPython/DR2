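; Procedural building actor that drives a PCG graph to lay out a modular building from grid counts, floor count and piece dimensions.
; The construction script derives wall, building and roof sizes from those settings.
; It writes them to the PCG graph instance as named vector parameters for floor, wall, corner, trim and roof offsets and scales.
; A random-size branch exists but is disconnected, and the event graph is empty.
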(event EventBeginPlay)

(event Collision|EventActorBeginOverlap
  (params (OtherActor :type Actor%20Object%20Reference)))

(event EventTick
  (params (DeltaSeconds :type Float%20%28single-precision%29)))

(fn ConstructionScript
  (bind _floorscale (Variables|Default|GetFloorScale))
  (bind _wallwidth (Variables|Default|GetWallWidth))
  (bind _wallthicknes (Variables|Default|GetWallThicknes))
  (bind _wallthicknes_2 (Variables|Default|GetWallThicknes))
  (bind _roofcornerwidth (Variables|Default|GetRoofCornerWidth))
  (bind _wallwidth_2 (Variables|Default|GetWallWidth))
  (bind _returnvalue (* _wallthicknes_2 2.0))
  (bind _returnvalue_2 (* _roofcornerwidth 2.0))
  (bind _returnvalue_3 (/ _wallwidth_2 _floorscale))
  (bind _returnvalue_4 (/ _wallwidth 2.0))
  (Utilities|FlowControl|Sequence
    (:then_1
      (LocalVariables|SetGraphInstance (Variables|/Script/PCG.PCGComponent|GetGraphInstance (Variables|Default|GetPCG)))
      (LocalVariables|SetTotalWallSize (Math|Vector2D|MakeVector2D (* (Variables|Default|GetWallWidth) (Variables|Default|GetBuildingGridCountX)) (* (Variables|Default|GetWallWidth) (Variables|Default|GetBuildingGridCountY))))
      (bind _output_get (LocalVariables|SetWallHalfWidth (/ (Variables|Default|GetWallWidth) 2.0)))
      (LocalVariables|SetNegativeWallHalfWidth (* _output_get -1.0))
      (LocalVariables|SetBuildingWallHeight (+ (* (Variables|Default|GetWallHeight) (- (Variables|Default|GetNumberOfFloors) 1)) (Variables|Default|GetTopWallHeight)))
      (LocalVariables|SetTotalBuildingSize (Math|Vector2D|MakeVector2D (+ (.x (LocalVariables|GetTotalWallSize)) _returnvalue) (+ (.y (LocalVariables|GetTotalWallSize)) _returnvalue)))
      (LocalVariables|SetTotal%20Building%20Height (+ (LocalVariables|GetBuildingWallHeight) (Variables|Default|GetRoofTrimHeight) (Variables|Default|GetRoofHeight))))
    (:then_2
      ;[0.15 0.15 0.15 0.5] Floor
      (Effects|Components|ParticleSystem|SetVectorParameter (LocalVariables|GetGraphInstance) "WallGrid_Extent" (Math|Vector|MakeVector (/ (.x (LocalVariables|GetTotalWallSize)) 2.0) (/ (.y (LocalVariables|GetTotalWallSize)) 2.0) 0.0))
      (Effects|Components|ParticleSystem|SetVectorParameter (LocalVariables|GetGraphInstance) "FloorScale" (Math|Vector|MakeVector _returnvalue_3 _returnvalue_3 1.0))
      (Effects|Components|ParticleSystem|SetVectorParameter (LocalVariables|GetGraphInstance) "Floor_Offset" (Math|Vector|MakeVector (* _returnvalue_4 -1.0) _returnvalue_4 1.0)))
    (:then_3
      ;[0.15 0.15 0.15 0.5] Walls
      (Effects|Components|ParticleSystem|SetVectorParameter (LocalVariables|GetGraphInstance) "WallOffset_1" (Math|Vector|MakeVector 0.0 (LocalVariables|GetWallHalfWidth) 0.0))
      (Effects|Components|ParticleSystem|SetVectorParameter (LocalVariables|GetGraphInstance) "WallOffset_2" (Math|Vector|MakeVector 0.0 (LocalVariables|GetNegativeWallHalfWidth) 0.0))
      (Effects|Components|ParticleSystem|SetVectorParameter (LocalVariables|GetGraphInstance) "WallOffset_3" (Math|Vector|MakeVector (LocalVariables|GetWallHalfWidth) 0.0 0.0))
      (Effects|Components|ParticleSystem|SetVectorParameter (LocalVariables|GetGraphInstance) "WallOffset_4" (Math|Vector|MakeVector (LocalVariables|GetNegativeWallHalfWidth) 0.0 0.0))
      (Effects|Components|ParticleSystem|SetVectorParameter (LocalVariables|GetGraphInstance) "WallOffsetAdjust" (Math|Vector|MakeVector (LocalVariables|GetNegativeWallHalfWidth) (Variables|Default|GetWallThicknes) 0.0)))
    (:then_4
      ;[0.15 0.15 0.15 0.5] Corners
      (Effects|Components|ParticleSystem|SetVectorParameter (LocalVariables|GetGraphInstance) "CornerOffset1" (Math|Vector|MakeVector (LocalVariables|GetNegativeWallHalfWidth) (LocalVariables|GetWallHalfWidth) 0.0))
      (Effects|Components|ParticleSystem|SetVectorParameter (LocalVariables|GetGraphInstance) "CornerOffset2" (Math|Vector|MakeVector (LocalVariables|GetNegativeWallHalfWidth) (LocalVariables|GetNegativeWallHalfWidth) 0.0))
      (Effects|Components|ParticleSystem|SetVectorParameter (LocalVariables|GetGraphInstance) "CornerOffset3" (Math|Vector|MakeVector (LocalVariables|GetWallHalfWidth) (LocalVariables|GetNegativeWallHalfWidth) 0.0))
      (Effects|Components|ParticleSystem|SetVectorParameter (LocalVariables|GetGraphInstance) "CornerOffset4" (Math|Vector|MakeVector (LocalVariables|GetWallHalfWidth) (LocalVariables|GetWallHalfWidth) 0.0))
      (Effects|Components|ParticleSystem|SetVectorParameter (LocalVariables|GetGraphInstance) "CornerOffsetAdjust" (Math|Vector|MakeVector (* _wallthicknes -1.0) _wallthicknes 0.0)))
    (:then_5
      ;[0.15 0.15 0.15 0.5] Roofcorner And Base
      (Effects|Components|ParticleSystem|SetVectorParameter (LocalVariables|GetGraphInstance) "lastWallPopintAdjust" (Math|Vector|MakeVector 0.0 0.0 (Utilities|Operators|Subtract (LocalVariables|GetBuildingWallHeight) (Variables|Default|GetWallHeight) (Variables|Default|GetTopWallHeight))))
      (Effects|Components|ParticleSystem|SetVectorParameter (LocalVariables|GetGraphInstance) "FirstWallPointAdjust" (Math|Vector|MakeVector 0.0 0.0 (Variables|Default|GetWallHeight)))
      (Effects|Components|ParticleSystem|SetVectorParameter (LocalVariables|GetGraphInstance) "BaseTrimAdjust" (Math|Vector|MakeVector 0.0 0.0 (Variables|Default|GetBaseWallHeight)))
      (Effects|Components|ParticleSystem|SetVectorParameter (LocalVariables|GetGraphInstance) "RooftrimAdjust" (Math|Vector|MakeVector 0.0 0.0 (LocalVariables|GetBuildingWallHeight)))
      (Effects|Components|ParticleSystem|SetVectorParameter (LocalVariables|GetGraphInstance) "RoofCornerAdjust" (Math|Vector|MakeVector 0.0 0.0 (+ (LocalVariables|GetBuildingWallHeight) (Variables|Default|GetRoofTrimHeight))))
      (Effects|Components|ParticleSystem|SetVectorParameter (LocalVariables|GetGraphInstance) "RoofCornerPivotAdjust" (Math|Vector|MakeVector 0.0 (* (Variables|Default|GetRoofCornerWidth) -1.0) 0.0)))
    (:then_6
      ;[0.15 0.15 0.15 0.5] Roof Horizontal And Vertical
      (LocalVariables|SetBuildingSpaceVertical (- (.x (LocalVariables|GetTotalBuildingSize)) _returnvalue_2))
      (LocalVariables|SetBuildingSpaceHorizontal (- (.y (LocalVariables|GetTotalBuildingSize)) _returnvalue_2))
      (Effects|Components|ParticleSystem|SetVectorParameter (LocalVariables|GetGraphInstance) "Last_Roof_Horizontal" (Math|Vector|MakeVector 0.0 (* (- (LocalVariables|GetBuildingSpaceHorizontal) (Variables|Default|GetRoofWidth)) -1.0) 0.0))
      (Effects|Components|ParticleSystem|SetVectorParameter (LocalVariables|GetGraphInstance) "Last_Roof_Vertical" (Math|Vector|MakeVector 0.0 (* (- (LocalVariables|GetBuildingSpaceVertical) (Variables|Default|GetRoofWidth)) -1.0) 0.0))
      (Effects|Components|ParticleSystem|SetVectorParameter (LocalVariables|GetGraphInstance) "RoofTopHeightAdjust" (Math|Vector|MakeVector 0.0 0.0 (LocalVariables|GetTotal%20Building%20Height)))
      (Effects|Components|ParticleSystem|SetVectorParameter (LocalVariables|GetGraphInstance) "RoofTopScaleAdjust" (Math|Vector|MakeVector (/ (LocalVariables|GetBuildingSpaceVertical) (Variables|Default|GetRoofTopSize)) (/ (LocalVariables|GetBuildingSpaceHorizontal) (Variables|Default|GetRoofTopSize)) 1.0))
      (Effects|Components|ParticleSystem|SetVectorParameter (LocalVariables|GetGraphInstance) "RoofTopOffsetAdjust" (Math|Vector|MakeVector (* (/ (LocalVariables|GetBuildingSpaceVertical) 2.0) -1.0) (/ (LocalVariables|GetBuildingSpaceHorizontal) 2.0) 0.0)))
    (:then_7
      (Effects|Components|ParticleSystem|SetVectorParameter (LocalVariables|GetGraphInstance) "TopFloorHeight" (Math|Vector|MakeVector 0.0 0.0 (- (LocalVariables|GetBuildingWallHeight) (Variables|Default|GetTopWallHeight)))))))