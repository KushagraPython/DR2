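; BP_MinePickUp is a racing pickup that adds one mine to the player or AI car that overlaps its sphere.
; The overlap casts to the player or AI pawn, and a DoOnce on each branch increments that car's mine count.
; The player branch plays a pickup sound and removes mesh and sphere, while the AI branch removes only the sphere.
; Both destroy the actor two seconds later.
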(event OnComponentBeginOverlap(Sphere)
  (params (OverlappedComponent :type Primitive%20Component%20Object%20Reference) (OtherActor :type Actor%20Object%20Reference) (OtherComp :type Primitive%20Component%20Object%20Reference) (OtherBodyIndex :type Integer) (bFromSweep :type Boolean) (SweepResult :type Hit%20Result%20Structure%20%28by%20ref%29))
  ;[1 1 1] When the player or AI overlap a mine pickup, +1 mine is added.
  (bind _asbp_offroad_car_pawn (Utilities|Casting|CastToBP_OffroadCar_Pawn OtherActor)
    (:then
      (Utilities|FlowControl|DoOnce false
        (:Completed
          (Variables|/Game/DerbyRacingTemplate/Blueprints/BP_OffroadCar_Pawn.BP_OffroadCar_Pawn_C|SetMine _asbp_offroad_car_pawn (+ (Variables|/Game/DerbyRacingTemplate/Blueprints/BP_OffroadCar_Pawn.BP_OffroadCar_Pawn_C|GetMine _asbp_offroad_car_pawn) 1))
          (Audio|Components|Audio|Play (Variables|Default|GetArmor_PickUp) 0.0)
          (Components|DestroyComponent (Variables|Default|GetSM_Cylinder))
          (Utilities|FlowControl|Delay 2.0)
          (Actor|DestroyActor))))
    (:CastFailed
      (bind _asbp_offroad_car_pawn_ai (Utilities|Casting|CastToBP_OffroadCar_PawnAI OtherActor))
      (Utilities|FlowControl|DoOnce false
        (:Completed
          (Variables|/Game/DerbyRacingTemplate/Blueprints/BP_OffroadCar_PawnAI.BP_OffroadCar_PawnAI_C|SetMines _asbp_offroad_car_pawn_ai (+ (Variables|/Game/DerbyRacingTemplate/Blueprints/BP_OffroadCar_PawnAI.BP_OffroadCar_PawnAI_C|GetMines _asbp_offroad_car_pawn_ai) 1))
          (Components|DestroyComponent (Variables|Default|GetSphere))
          (Utilities|FlowControl|Delay 2.0)
          (Actor|DestroyActor))))))

(fn ConstructionScript)