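; BP_ArmorPickUp is a derby racing pickup that restores armor to full for a player or AI offroad car.
; On sphere overlap it casts to the player or AI car pawn and, if armor is below the cap, sets it to maximum once.
; The pickup sound or effect plays only for the player; both paths then remove the fire effect and sphere and destroy the actor after a short delay.
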(event OnComponentBeginOverlap(Sphere)
  (params (OverlappedComponent :type Primitive%20Component%20Object%20Reference) (OtherActor :type Actor%20Object%20Reference) (OtherComp :type Primitive%20Component%20Object%20Reference) (OtherBodyIndex :type Integer) (bFromSweep :type Boolean) (SweepResult :type Hit%20Result%20Structure%20%28by%20ref%29))
  ;[1 1 1] When the player or AI overlap an armored pickup, +100 armor is credited, provided that the armor is less than 100 .
  (bind _asbp_offroad_car_pawn (Utilities|Casting|CastToBP_OffroadCar_Pawn OtherActor)
    (:then
      (bind _output_get (Variables|Default|SetAs%20Offroad%20Car%20Pawn _asbp_offroad_car_pawn))
      (if (< (Variables|/Game/DerbyRacingTemplate/Blueprints/BP_OffroadCar_Pawn.BP_OffroadCar_Pawn_C|GetArmor _output_get) 1e+02)
        (Utilities|FlowControl|DoOnce false
          (:Completed
            (Variables|/Game/DerbyRacingTemplate/Blueprints/BP_OffroadCar_Pawn.BP_OffroadCar_Pawn_C|SetArmor (Variables|Default|GetAs%20Offroad%20Car%20Pawn) 1e+02)
            (Audio|Components|Audio|Play (Variables|Default|GetArmorPickUp) 0.0)
            (Components|DestroyComponent (Variables|Default|GetNS_SttylizedFireGreen) :!label _label)
            (Utilities|FlowControl|Delay 2.0)
            (Actor|DestroyActor)))))
    (:CastFailed
      (bind _asbp_offroad_car_pawn_ai (Utilities|Casting|CastToBP_OffroadCar_PawnAI OtherActor))
      (if (< (Variables|/Game/DerbyRacingTemplate/Blueprints/BP_OffroadCar_PawnAI.BP_OffroadCar_PawnAI_C|GetArmor _asbp_offroad_car_pawn_ai) 1e+02)
        (Utilities|FlowControl|DoOnce false
          (:Completed
            (Variables|/Game/DerbyRacingTemplate/Blueprints/BP_OffroadCar_PawnAI.BP_OffroadCar_PawnAI_C|SetArmor _asbp_offroad_car_pawn_ai 1e+02)
            (goto _label)))))))

(fn ConstructionScript)