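; BP_Mine is a mine hazard for the derby racing template that explodes when something overlaps its sphere.
; For player or AI off-road cars, a one-shot hit takes 100 armor, or 100 health when armor is under 100, exploding only if that damage applies.
; Any other overlapping actor detonates it directly.
; The explosion activates Niagara and sound effects, removes the sphere and idle effect, then destroys the actor after a delay.
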(event OnComponentBeginOverlap(Sphere)
  (params (OverlappedComponent :type Primitive%20Component%20Object%20Reference) (OtherActor :type Actor%20Object%20Reference) (OtherComp :type Primitive%20Component%20Object%20Reference) (OtherBodyIndex :type Integer) (bFromSweep :type Boolean) (SweepResult :type Hit%20Result%20Structure%20%28by%20ref%29))
  ;[1 1 1] When the player or AI overlap a mine, then if armor = 100, then - 100 armor, and if armor = 0 then - 100 health.
  (bind _asbp_offroad_car_pawn (Utilities|Casting|CastToBP_OffroadCar_Pawn OtherActor)
    (:then
      (Variables|Default|SetAs%20Offroad%20Car%20Pawn _asbp_offroad_car_pawn)
      (if (>= (Variables|/Game/DerbyRacingTemplate/Blueprints/BP_OffroadCar_Pawn.BP_OffroadCar_Pawn_C|GetArmor (Variables|Default|GetAs%20Offroad%20Car%20Pawn)) 1e+02)
        (Utilities|FlowControl|DoOnce false
          (:Completed
            (Variables|/Game/DerbyRacingTemplate/Blueprints/BP_OffroadCar_Pawn.BP_OffroadCar_Pawn_C|SetArmor (Variables|Default|GetAs%20Offroad%20Car%20Pawn) (- (Variables|/Game/DerbyRacingTemplate/Blueprints/BP_OffroadCar_Pawn.BP_OffroadCar_Pawn_C|GetArmor (Variables|Default|GetAs%20Offroad%20Car%20Pawn)) 1e+02))
            (CallFunction|ExplosionEvent)))
        (else
          (Utilities|FlowControl|DoOnce false
            (:Completed
              (if (>= (Variables|/Game/DerbyRacingTemplate/Blueprints/BP_OffroadCar_Pawn.BP_OffroadCar_Pawn_C|GetHealth (Variables|Default|GetAs%20Offroad%20Car%20Pawn)) 1e+02)
                (bind _output_get (Variables|/Game/DerbyRacingTemplate/Blueprints/BP_OffroadCar_Pawn.BP_OffroadCar_Pawn_C|SetHealth (Variables|Default|GetAs%20Offroad%20Car%20Pawn) (- (Variables|/Game/DerbyRacingTemplate/Blueprints/BP_OffroadCar_Pawn.BP_OffroadCar_Pawn_C|GetHealth (Variables|Default|GetAs%20Offroad%20Car%20Pawn)) 1e+02)))
                (Development|PrintString (Utilities|String|ToString(Float) _output_get) true true "(R=1.000000,G=0.121361,B=0.000000,A=1.000000)")
                (CallFunction|ExplosionEvent)))))))
    (:CastFailed
      (bind _asbp_offroad_car_pawn_ai (Utilities|Casting|CastToBP_OffroadCar_PawnAI OtherActor)
        (:then
          (Variables|Default|SetAs%20Offroad%20Car%20Pawn%20AI _asbp_offroad_car_pawn_ai)
          (if (>= (Variables|/Game/DerbyRacingTemplate/Blueprints/BP_OffroadCar_PawnAI.BP_OffroadCar_PawnAI_C|GetArmor (Variables|Default|GetAs%20Offroad%20Car%20Pawn%20AI)) 1e+02)
            (Utilities|FlowControl|DoOnce false
              (:Completed
                (Variables|/Game/DerbyRacingTemplate/Blueprints/BP_OffroadCar_PawnAI.BP_OffroadCar_PawnAI_C|SetArmor (Variables|Default|GetAs%20Offroad%20Car%20Pawn%20AI) (- (Variables|/Game/DerbyRacingTemplate/Blueprints/BP_OffroadCar_PawnAI.BP_OffroadCar_PawnAI_C|GetArmor (Variables|Default|GetAs%20Offroad%20Car%20Pawn%20AI)) 1e+02))
                (CallFunction|ExplosionEvent)))
            (else
              (Utilities|FlowControl|DoOnce false
                (:Completed
                  (if (>= (Variables|/Game/DerbyRacingTemplate/Blueprints/BP_OffroadCar_PawnAI.BP_OffroadCar_PawnAI_C|GetHealth (Variables|Default|GetAs%20Offroad%20Car%20Pawn%20AI)) 1e+02)
                    (bind _output_get_2 (Variables|/Game/DerbyRacingTemplate/Blueprints/BP_OffroadCar_PawnAI.BP_OffroadCar_PawnAI_C|SetHealth (Variables|Default|GetAs%20Offroad%20Car%20Pawn%20AI) (- (Variables|/Game/DerbyRacingTemplate/Blueprints/BP_OffroadCar_PawnAI.BP_OffroadCar_PawnAI_C|GetHealth (Variables|Default|GetAs%20Offroad%20Car%20Pawn%20AI)) 1e+02)))
                    (Development|PrintString (Utilities|String|ToString(Float) _output_get_2) true true "(R=1.000000,G=0.121361,B=0.000000,A=1.000000)")
                    (CallFunction|ExplosionEvent)))))))
        (:CastFailed
          (CallFunction|ExplosionEvent))))))

(event Custom|ExplosionEvent
  ;[1 1 1] Explosion logic
  (Components|Activation|SetActive (Variables|Default|GetNS_Explosion) true false)
  (Utilities|IsValid (Variables|Default|GetSphere)
    (:Is%20Valid
      (Components|DestroyComponent (Variables|Default|GetNS_PixelFireCrossBig))
      (Audio|Components|Audio|Play (Variables|Default|GetExplosion_Cue) 0.0)
      (Utilities|FlowControl|Delay 1e+01)
      (Actor|DestroyActor) ; Then destroy this projectile
    )))

(fn ConstructionScript)