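; Rotating rocket launcher pickup for derby racing that arms player and AI offroad cars.
; Separate overlap spheres for player and AI pawns run mirrored do-once logic, enabling the first or second launcher, disabling the mortar and adding rockets.
; It then plays a sound, destroys its own components and, after a delay, spawns a replacement copy without destroying the original actor.
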(event OnComponentBeginOverlap(Sphere)
  (params (OverlappedComponent :type Primitive%20Component%20Object%20Reference) (OtherActor :type Actor%20Object%20Reference) (OtherComp :type Primitive%20Component%20Object%20Reference) (OtherBodyIndex :type Integer) (bFromSweep :type Boolean) (SweepResult :type Hit%20Result%20Structure%20%28by%20ref%29))
  ;[1 1 1] When the player runs into a rocket launcher pickup, then if no rocket launcher has been pickuped before, one rocket launcher will be activated, if one has already been found, then two rocket launchers will be activated.
  (bind _asbp_offroad_car_pawn (Utilities|Casting|CastToBP_OffroadCar_Pawn OtherActor))
  (Variables|Default|SetAs%20Offroad%20Car%20Pawn _asbp_offroad_car_pawn)
  (Utilities|FlowControl|DoOnce false :!label _label
    (:Completed
      (if (Variables|/Game/DerbyRacingTemplate/Blueprints/BP_OffroadCar_Pawn.BP_OffroadCar_Pawn_C|GetOneRLWasPickedUp (Variables|Default|GetAs%20Offroad%20Car%20Pawn))
        (Variables|/Game/DerbyRacingTemplate/Blueprints/BP_OffroadCar_Pawn.BP_OffroadCar_Pawn_C|SetTwoRLActive (Variables|Default|GetAs%20Offroad%20Car%20Pawn) true :!label _label_2)
        (Variables|/Game/DerbyRacingTemplate/Blueprints/BP_OffroadCar_Pawn.BP_OffroadCar_Pawn_C|SetTwoRLWasPickedUp (Variables|Default|GetAs%20Offroad%20Car%20Pawn) true)
        (Variables|/Game/DerbyRacingTemplate/Blueprints/BP_OffroadCar_Pawn.BP_OffroadCar_Pawn_C|SetOneRLActive (Variables|Default|GetAs%20Offroad%20Car%20Pawn) false)
        (Variables|/Game/DerbyRacingTemplate/Blueprints/BP_OffroadCar_Pawn.BP_OffroadCar_Pawn_C|SetMortarActive (Variables|Default|GetAs%20Offroad%20Car%20Pawn) false)
        (Rendering|SetVisibility (Variables|/Game/DerbyRacingTemplate/Blueprints/BP_OffroadCar_Pawn.BP_OffroadCar_Pawn_C|GetSM_RL2 (Variables|Default|GetAs%20Offroad%20Car%20Pawn)) true false)
        (elif (Variables|/Game/DerbyRacingTemplate/Blueprints/BP_OffroadCar_Pawn.BP_OffroadCar_Pawn_C|GetTwoRLActive (Variables|Default|GetAs%20Offroad%20Car%20Pawn))
          (goto _label_2)
          (elif (Variables|/Game/DerbyRacingTemplate/Blueprints/BP_OffroadCar_Pawn.BP_OffroadCar_Pawn_C|GetOneRLActive (Variables|Default|GetAs%20Offroad%20Car%20Pawn))
            (goto _label_2)
            (else
              (Variables|/Game/DerbyRacingTemplate/Blueprints/BP_OffroadCar_Pawn.BP_OffroadCar_Pawn_C|SetOneRLActive (Variables|Default|GetAs%20Offroad%20Car%20Pawn) true)
              (Variables|/Game/DerbyRacingTemplate/Blueprints/BP_OffroadCar_Pawn.BP_OffroadCar_Pawn_C|SetOneRLWasPickedUp (Variables|Default|GetAs%20Offroad%20Car%20Pawn) true)
              (Rendering|SetVisibility (Variables|/Game/DerbyRacingTemplate/Blueprints/BP_OffroadCar_Pawn.BP_OffroadCar_Pawn_C|GetSM_RL1 (Variables|Default|GetAs%20Offroad%20Car%20Pawn)) true false)
              (Variables|/Game/DerbyRacingTemplate/Blueprints/BP_OffroadCar_Pawn.BP_OffroadCar_Pawn_C|SetMortarActive (Variables|Default|GetAs%20Offroad%20Car%20Pawn) false)))))
      (Variables|/Game/DerbyRacingTemplate/Blueprints/BP_OffroadCar_Pawn.BP_OffroadCar_Pawn_C|SetRockets (Variables|Default|GetAs%20Offroad%20Car%20Pawn) (+ (Variables|/Game/DerbyRacingTemplate/Blueprints/BP_OffroadCar_Pawn.BP_OffroadCar_Pawn_C|GetRockets (Variables|Default|GetAs%20Offroad%20Car%20Pawn)) 10))
      (Components|DestroyComponent (Variables|Default|GetSphere))
      (Audio|Components|Audio|Play (Variables|Default|GetRL_PickUp) 0.0)
      (Utilities|FlowControl|Delay 2.0)
      (Components|DestroyComponent (Variables|Default|GetSphere1))
      (Utilities|FlowControl|Delay 3e+01)
      (Game|SpawnActorfromClass "BP_RocketLauncherPickUp_C" (Transformation|GetActorTransform) "Undefined" "MultiplyWithRoot" 0 0)
      (goto _label Reset))))

(event OnComponentBeginOverlap(Sphere1)
  (params (OverlappedComponent :type Primitive%20Component%20Object%20Reference) (OtherActor :type Actor%20Object%20Reference) (OtherComp :type Primitive%20Component%20Object%20Reference) (OtherBodyIndex :type Integer) (bFromSweep :type Boolean) (SweepResult :type Hit%20Result%20Structure%20%28by%20ref%29))
  (bind _sphere1 (Variables|Default|GetSphere1))
  (bind _sphere (Variables|Default|GetSphere))
  (bind _sm_rl1 (Variables|Default|GetSM_RL1))
  (bind _rl_pickup (Variables|Default|GetRL_PickUp))
  ;[1 1 1] When the AI runs into a rocket launcher pickup, then if no rocket launcher has been pickuped before, one rocket launcher will be activated, if one has already been found, then two rocket launchers will be activated.
  (bind _asbp_offroad_car_pawn_ai (Utilities|Casting|CastToBP_OffroadCar_PawnAI OtherActor))
  (Variables|Default|SetAs%20Offroad%20Car%20Pawn%20AI _asbp_offroad_car_pawn_ai)
  (Utilities|FlowControl|DoOnce false :!label _label
    (:Completed
      (if (Variables|/Game/DerbyRacingTemplate/Blueprints/BP_OffroadCar_PawnAI.BP_OffroadCar_PawnAI_C|GetOneRLWasPickedUp (Variables|Default|GetAs%20Offroad%20Car%20Pawn%20AI))
        (Variables|/Game/DerbyRacingTemplate/Blueprints/BP_OffroadCar_PawnAI.BP_OffroadCar_PawnAI_C|SetTwoRLActive (Variables|Default|GetAs%20Offroad%20Car%20Pawn%20AI) true :!label _label_2)
        (Variables|/Game/DerbyRacingTemplate/Blueprints/BP_OffroadCar_PawnAI.BP_OffroadCar_PawnAI_C|SetTwoRLWasPickedUp (Variables|Default|GetAs%20Offroad%20Car%20Pawn%20AI) true)
        (Variables|/Game/DerbyRacingTemplate/Blueprints/BP_OffroadCar_PawnAI.BP_OffroadCar_PawnAI_C|SetOneRLActive (Variables|Default|GetAs%20Offroad%20Car%20Pawn%20AI) false)
        (Variables|/Game/DerbyRacingTemplate/Blueprints/BP_OffroadCar_PawnAI.BP_OffroadCar_PawnAI_C|SetMortarActive (Variables|Default|GetAs%20Offroad%20Car%20Pawn%20AI) false)
        (Rendering|SetVisibility (Variables|/Game/DerbyRacingTemplate/Blueprints/BP_OffroadCar_PawnAI.BP_OffroadCar_PawnAI_C|GetSM_RL2 (Variables|Default|GetAs%20Offroad%20Car%20Pawn%20AI)) true false)
        (elif (Variables|/Game/DerbyRacingTemplate/Blueprints/BP_OffroadCar_PawnAI.BP_OffroadCar_PawnAI_C|GetTwoRLActive (Variables|Default|GetAs%20Offroad%20Car%20Pawn%20AI))
          (goto _label_2)
          (elif (Variables|/Game/DerbyRacingTemplate/Blueprints/BP_OffroadCar_PawnAI.BP_OffroadCar_PawnAI_C|GetOneRLActive (Variables|Default|GetAs%20Offroad%20Car%20Pawn%20AI))
            (goto _label_2)
            (else
              (Variables|/Game/DerbyRacingTemplate/Blueprints/BP_OffroadCar_PawnAI.BP_OffroadCar_PawnAI_C|SetOneRLActive (Variables|Default|GetAs%20Offroad%20Car%20Pawn%20AI) true)
              (Variables|/Game/DerbyRacingTemplate/Blueprints/BP_OffroadCar_PawnAI.BP_OffroadCar_PawnAI_C|SetOneRLWasPickedUp (Variables|Default|GetAs%20Offroad%20Car%20Pawn%20AI) true)
              (Rendering|SetVisibility (Variables|/Game/DerbyRacingTemplate/Blueprints/BP_OffroadCar_PawnAI.BP_OffroadCar_PawnAI_C|GetSM_RL1 (Variables|Default|GetAs%20Offroad%20Car%20Pawn%20AI)) true false)
              (Variables|/Game/DerbyRacingTemplate/Blueprints/BP_OffroadCar_PawnAI.BP_OffroadCar_PawnAI_C|SetMortarActive (Variables|Default|GetAs%20Offroad%20Car%20Pawn%20AI) false)))))
      (Variables|/Game/DerbyRacingTemplate/Blueprints/BP_OffroadCar_PawnAI.BP_OffroadCar_PawnAI_C|SetRockets (Variables|Default|GetAs%20Offroad%20Car%20Pawn%20AI) (+ (Variables|/Game/DerbyRacingTemplate/Blueprints/BP_OffroadCar_PawnAI.BP_OffroadCar_PawnAI_C|GetRockets (Variables|Default|GetAs%20Offroad%20Car%20Pawn%20AI)) 10))
      (Utilities|IsValid _sm_rl1
        (:Is%20Valid
          (Components|DestroyComponent _sm_rl1))
        (:Is%20Not%20Valid
          _))
      (Utilities|IsValid _sphere
        (:Is%20Valid
          (Components|DestroyComponent _sphere))
        (:Is%20Not%20Valid
          _))
      (Audio|Components|Audio|Play (Variables|Default|GetRL_PickUp) 0.0)
      (Utilities|FlowControl|Delay 2.0)
      (Utilities|IsValid _rl_pickup
        (:Is%20Valid
          (Components|DestroyComponent _rl_pickup)
          (Utilities|IsValid _sphere1
            (:Is%20Valid
              (Components|DestroyComponent _sphere1)
              (Utilities|FlowControl|Delay 3e+01)
              (Game|SpawnActorfromClass "BP_RocketLauncherPickUp_C" (Transformation|GetActorTransform) "Undefined" "MultiplyWithRoot" 0 0)
              (goto _label Reset))))))))

(event EventBeginPlay
  ;[1 1 1] Rotation
  (AddComponent|AddRotatingMovementComponent))

(fn ConstructionScript)